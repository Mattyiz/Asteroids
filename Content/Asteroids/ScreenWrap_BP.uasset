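; Screen-wrap component for the Asteroids game that teleports parts of its owning actor across the play field when they leave it.
; Every Tick it loops over the owner's static mesh components tagged "wrap" and checks each world location against fixed X and Y bounds.
; Out-of-bounds meshes get that coordinate negated with a small inward nudge, landing just inside the opposite edge.
; It moves the mesh components themselves, leaving Z unchanged.
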(event `self.ReceiveTick`
  (params (DeltaSeconds :type "Float (single-precision)"))
  (bind _returnvalue (`Actor.GetComponentsByTag` (`self.GetOwner`) "/Script/Engine.StaticMeshComponent" "wrap"))
  (for (_ _array_index) _returnvalue
    (`|ExecutionSequence`
      (:`then_0`
        (bind _output (`|GetArrayItem` _returnvalue _array_index))
        (bind (_returnvalue_x _returnvalue_y _returnvalue_z) (`KismetMathLibrary.BreakVector` (`SceneComponent.K2_GetComponentLocation` _output)))
        (if (> _returnvalue_x 2450.0)
          (`SceneComponent.K2_SetWorldLocation` _output (`KismetMathLibrary.MakeVector` (+ (* _returnvalue_x -1.0) 10.0) _returnvalue_y _returnvalue_z) false false)))
      (:`then_1`
        (if (< _returnvalue_x -2450.0)
          (`SceneComponent.K2_SetWorldLocation` _output (`KismetMathLibrary.MakeVector` (- (* _returnvalue_x -1.0) 10.0) _returnvalue_y _returnvalue_z) false false)))
      (:`then_2`
        (if (> _returnvalue_y 3050.0)
          (`SceneComponent.K2_SetWorldLocation` _output (`KismetMathLibrary.MakeVector` _returnvalue_x (+ (* _returnvalue_y -1.0) 10.0) _returnvalue_z) false false)))
      (:`then_3`
        (if (< _returnvalue_y -3050.0)
          (`SceneComponent.K2_SetWorldLocation` _output (`KismetMathLibrary.MakeVector` _returnvalue_x (- (* _returnvalue_y -1.0) 10.0) _returnvalue_z) false false))))))