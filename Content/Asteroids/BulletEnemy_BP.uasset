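; Enemy bullet actor for an Asteroids game that flies in a random direction and then removes itself.
; BeginPlay picks a random, unnormalized XY direction, so travel speed varies between bullets.
; Tick offsets the Sphere component by Direction times Speed without sweep or delta-time scaling, making movement frame-rate dependent.
; A Delay on the Tick chain destroys the actor about 0.8 seconds after the first tick.
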(event `self.ReceiveBeginPlay`
  (set `self.Direction` (`KismetMathLibrary.MakeVector` (`KismetMathLibrary.RandomFloatInRange` -1.0 1.0) (`KismetMathLibrary.RandomFloatInRange` -1.0 1.0))))

(event `self.ReceiveTick`
  (params (DeltaSeconds :type "Float (single-precision)"))
  (`SceneComponent.K2_AddWorldOffset` (`self.Sphere`) (* (`self.Direction`) (`self.Speed`)) false false)
  (`KismetSystemLibrary.Delay` 0.8)
  (`self.K2_DestroyActor`))

(fn `UserConstructionScript`
  (`parent.UserConstructionScript`))