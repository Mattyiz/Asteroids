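; Comet actor for the Asteroids game that aims at the player and awards points when its Destroy function is called.
; On BeginPlay it sets Speed and a Direction toward the player's second "wrap"-tagged mesh with slight random X/Y jitter, then removes itself after a short delay.
; Tick only calls the parent, with no movement logic here.
; Destroy adds a bonus to both GameManager score counters before removing the actor.
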(event `self.ReceiveBeginPlay`
  (set `self.Speed` 0.01)
  (bind _outactors (`GameplayStatics.GetAllActorsOfClass` "/Game/Asteroids/Player_BP.Player_BP_C"))
  (bind _output_get (set `self.Player` (`|GetArrayItem` _outactors)))
  (bind (_returnvalue_x _returnvalue_y _returnvalue_z) (`KismetMathLibrary.BreakVector` (- (`SceneComponent.K2_GetComponentLocation` (`|GetArrayItem` (`self.GetComponentsByTag` _output_get "/Script/Engine.StaticMeshComponent" "wrap") 1)) (`self.K2_GetActorLocation`))))
  (set `self.Direction` (`KismetMathLibrary.MakeVector` (+ _returnvalue_x (`KismetMathLibrary.RandomFloatInRange` -2.0 2.0)) (+ _returnvalue_y (`KismetMathLibrary.RandomFloatInRange` -2.0 2.0)) _returnvalue_z))
  (`KismetSystemLibrary.Delay` 2.0)
  (`self.K2_DestroyActor`))

(event `self.ReceiveTick`
  (params (DeltaSeconds :type "Float (single-precision)"))
  (`parent.ReceiveTick` DeltaSeconds))

(fn `Destroy`
  (bind _outactors (`GameplayStatics.GetAllActorsOfClass` "/Game/Asteroids/GameManager_BP.GameManager_BP_C"))
  (bind _output_get (set `self.GameManager` (`|GetArrayItem` _outactors)))
  (set `/Game/Asteroids/GameManager_BP.ScoreSinceLife` (+ (`/Game/Asteroids/GameManager_BP.ScoreSinceLife` _output_get) 500) _output_get)
  (set `/Game/Asteroids/GameManager_BP.Score` (+ (`/Game/Asteroids/GameManager_BP.Score` _output_get) 500) _output_get)
  (`self.K2_DestroyActor`))

(fn `UserConstructionScript`
  (`parent.UserConstructionScript`))