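; Player ship pawn for an Asteroids game that rotates, thrusts and shoots.
; Input drives physics torque and force on the Cone, and Shoot spawns a bullet at the BulletSpawner.
; BeginPlay spawns three offset Lives actors as a life display.
; Asteroid overlaps on the HitBox start brief invincibility, counted down in Tick, and either remove a life marker and teleport the Cone to world origin or destroy the player.
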(event `InputAxis|Rotate`
  (params (AxisValue :type "Float (single-precision)"))
  (`PrimitiveComponent.AddTorqueInDegrees` (`self.Cone`) (`KismetMathLibrary.MakeVector` 0.0 0.0 (* AxisValue 500.0)) "None" true))

(event `InputAxis|Forward`
  (params (AxisValue :type "Float (single-precision)"))
  (bind _cone (`self.Cone`))
  (`PrimitiveComponent.AddForce` _cone (* (`SceneComponent.GetUpVector` _cone) (* AxisValue 650.0)) "None" true))

(event `InputAction|Shoot`
  (params (Key :type "Key Structure"))
  (:`Pressed`
    (`|SpawnActorFromClass` "/Game/Asteroids/Bullet_BP.Bullet_BP_C" (`SceneComponent.K2_GetComponentToWorld` (`self.BulletSpawner`)) "AdjustIfPossibleButAlwaysSpawn" "MultiplyWithRoot" null null)))

(event `self.ReceiveBeginPlay`
  (bind _returnvalue (`SceneComponent.K2_GetComponentToWorld` (`self.LiveSpawner`)))
  (bind _returnvalue_2 (`SceneComponent.K2_GetComponentToWorld` (`self.LiveSpawner`)))
  (bind _returnvalue_3 (`|SpawnActorFromClass` "/Game/Asteroids/Lives.Lives_C" (`SceneComponent.K2_GetComponentToWorld` (`self.LiveSpawner`)) "AlwaysSpawn" "MultiplyWithRoot" null null))
  (bind _returnvalue_4 (`|SpawnActorFromClass` "/Game/Asteroids/Lives.Lives_C" (`KismetMathLibrary.MakeTransform` (`KismetMathLibrary.MakeVector` (.x (.location _returnvalue_2)) (- (.y (.location _returnvalue_2)) 60.0) (.z (.location _returnvalue_2))) (.rotation _returnvalue_2) (.scale _returnvalue_2)) "AlwaysSpawn" "MultiplyWithRoot" null null))
  (bind _returnvalue_5 (`|SpawnActorFromClass` "/Game/Asteroids/Lives.Lives_C" (`KismetMathLibrary.MakeTransform` (`KismetMathLibrary.MakeVector` (.x (.location _returnvalue)) (- (.y (.location _returnvalue)) 120.0) (.z (.location _returnvalue))) (.rotation _returnvalue) (.scale _returnvalue)) "AlwaysSpawn" "MultiplyWithRoot" null null)))

(event `self.HitBox.OnComponentBeginOverlap`
  (params (OverlappedComponent :type "PrimitiveComponent Object Reference") (OtherActor :type "Actor Object Reference") (OtherComp :type "PrimitiveComponent Object Reference") (OtherBodyIndex :type Integer) (bFromSweep :type Boolean) (SweepResult :type "HitResult Structure (by ref)"))
  (cast `/Game/Asteroids/AsteriodParent_BP` OtherActor)
  (if (not (> (`self.Invincibility`) 0.0))
    (set `self.Invincibility` 1.0)
    (bind _output_get (set `self.Lives` (- (`self.Lives`) 1)))
    (if (>= _output_get 0)
      (bind _array (`|MakeArray` (stale `self.ReceiveBeginPlay` _returnvalue_3) (stale `self.ReceiveBeginPlay` _returnvalue_4) (stale `self.ReceiveBeginPlay` _returnvalue_5)))
      (`self.K2_DestroyActor` (`|GetArrayItem` _array (`self.Lives`)))
      (`KismetArrayLibrary.Array_Remove` _array (`self.Lives`))
      (`SceneComponent.K2_SetWorldLocation` (`self.Cone`) (0.0 0.0 0.0) false false)
      (else
        (`self.K2_DestroyActor`)))))

(event `self.ReceiveTick`
  (params (DeltaSeconds :type "Float (single-precision)"))
  (if (> (`self.Invincibility`) 0.0)
    (set `self.Invincibility` (- (`self.Invincibility`) DeltaSeconds))))

(fn `UserConstructionScript`)