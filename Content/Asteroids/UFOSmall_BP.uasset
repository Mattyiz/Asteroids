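; Small UFO enemy for an Asteroids game that flies along a set direction, fires accurate enemy bullets and awards points when destroyed.
; Tick offsets the base by Direction times Speed without delta-time scaling, then uses a Delay to spawn a BulletEnemyAccurate_BP at the Sphere roughly once per second.
; Destroy adds a fixed bonus to the GameManager_BP's Score and ScoreSinceLife before removing the actor.
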(event `self.ReceiveTick`
  (params (DeltaSeconds :type "Float (single-precision)"))
  (bind (_returnvalue_location _returnvalue_rotation) (`KismetMathLibrary.BreakTransform` (`SceneComponent.K2_GetComponentToWorld` (`self.Sphere`))))
  (`SceneComponent.K2_AddWorldOffset` (`self.Base`) (* (`self.Direction`) (`self.Speed`)) false false)
  (`KismetSystemLibrary.Delay` 1.0)
  (`|SpawnActorFromClass` "/Game/Asteroids/BulletEnemyAccurate_BP.BulletEnemyAccurate_BP_C" (`KismetMathLibrary.MakeTransform` _returnvalue_location _returnvalue_rotation) "Undefined" "MultiplyWithRoot" null null))

(fn `Destroy`
  (bind _outactors (`GameplayStatics.GetAllActorsOfClass` "/Game/Asteroids/GameManager_BP.GameManager_BP_C"))
  (bind _output (`|GetArrayItem` _outactors))
  (set `/Game/Asteroids/GameManager_BP.ScoreSinceLife` (+ (`/Game/Asteroids/GameManager_BP.ScoreSinceLife` _output) 1000) _output)
  (set `/Game/Asteroids/GameManager_BP.Score` (+ (`/Game/Asteroids/GameManager_BP.Score` _output) 1000) _output)
  (`self.K2_DestroyActor`))

(fn `UserConstructionScript`
  (`parent.UserConstructionScript`))