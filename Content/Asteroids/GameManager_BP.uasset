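; Game manager for an Asteroids game that spawns asteroid waves and periodic hazards.
; It spawns five asteroids at BeginPlay and again whenever Tick finds none left.
; A randomized countdown in DecideSpawns picks UFO, comet or small UFO by rising Score tier, placing each by rejection sampling outside a central band on both axes.
; Tick also wraps ScoreSinceLife at its threshold, without granting a life here.
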(event `self.ReceiveBeginPlay`
  (`self.SpawnAsteroids`)
  (`self.SpawnAsteroids`)
  (`self.SpawnAsteroids`)
  (`self.SpawnAsteroids`)
  (`self.SpawnAsteroids`)
  (set `self.SpawnTimer` 10.0))

(event `self.ReceiveTick`
  (params (DeltaSeconds :type "Float (single-precision)"))
  (`self.DecideSpawns` DeltaSeconds)
  (bind _outactors (`GameplayStatics.GetAllActorsOfClass` "/Game/Asteroids/AsteriodParent_BP.AsteriodParent_BP_C"))
  (if (<= (`KismetArrayLibrary.Array_Length` _outactors) 0)
    (`self.SpawnAsteroids`)
    (`self.SpawnAsteroids`)
    (`self.SpawnAsteroids`)
    (`self.SpawnAsteroids`)
    (`self.SpawnAsteroids`))
  (if (>= (`self.ScoreSinceLife`) 10000)
    (set `self.ScoreSinceLife` (- (`self.ScoreSinceLife`) 10000))))

(fn `DecideSpawns`
  (params (DeltaTime :type "Float (double-precision)"))
  (if (> (`self.SpawnTimer`) 0.0)
    (set `self.SpawnTimer` (- (`self.SpawnTimer`) DeltaTime))
    (else
      (set `self.SpawnTimer` (`KismetMathLibrary.RandomFloatInRange` 8.0 12.0))
      (if (>= (`self.Score`) 5000)
        (if (>= (`self.Score`) 15000)
          (`self.SpawnSmallUFO`)
          (else
            (`self.SpawnComet`)))
        (else
          (`self.SpawnUFO`))))))

(fn `SpawnAsteroids`
  (set `self.SpawnX` (`KismetMathLibrary.RandomFloatInRange` -2000.0 2000.0))
  (while (and (> (`self.SpawnX`) -1000.0) (< (`self.SpawnX`) 1000.0))
    (set `self.SpawnX` (`KismetMathLibrary.RandomFloatInRange` -2000.0 2000.0)))
  (set `self.SpawnY` (`KismetMathLibrary.RandomFloatInRange` -2500.0 2500.0))
  (while (and (> (`self.SpawnY`) -500.0) (< (`self.SpawnY`) 500.0))
    (set `self.SpawnY` (`KismetMathLibrary.RandomFloatInRange` -2500.0 2500.0)))
  (`|SpawnActorFromClass` "/Game/Asteroids/AsteriodParent_BP.AsteriodParent_BP_C" (`KismetMathLibrary.MakeTransform` (`KismetMathLibrary.MakeVector` (`self.SpawnX`) (`self.SpawnY`) 200.0)) "AdjustIfPossibleButAlwaysSpawn" "MultiplyWithRoot" null null))

(fn `SpawnComet`
  (set `self.SpawnX` (`KismetMathLibrary.RandomFloatInRange` -2000.0 2000.0))
  (while (and (> (`self.SpawnX`) -1500.0) (< (`self.SpawnX`) 1500.0))
    (set `self.SpawnX` (`KismetMathLibrary.RandomFloatInRange` -2000.0 2000.0)))
  (set `self.SpawnY` (`KismetMathLibrary.RandomFloatInRange` -2500.0 2500.0))
  (while (and (> (`self.SpawnY`) -2000.0) (< (`self.SpawnY`) 2000.0))
    (set `self.SpawnY` (`KismetMathLibrary.RandomFloatInRange` -2500.0 2500.0)))
  (`|SpawnActorFromClass` "/Game/Asteroids/Comet_BP.Comet_BP_C" (`KismetMathLibrary.MakeTransform` (`KismetMathLibrary.MakeVector` (`self.SpawnX`) (`self.SpawnY`) 200.0)) "Undefined" "MultiplyWithRoot" null null))

(fn `SpawnSmallUFO`
  (set `self.SpawnX` (`KismetMathLibrary.RandomFloatInRange` -2000.0 2000.0))
  (while (and (> (`self.SpawnX`) -1000.0) (< (`self.SpawnX`) 1000.0))
    (set `self.SpawnX` (`KismetMathLibrary.RandomFloatInRange` -2000.0 2000.0)))
  (set `self.SpawnY` (`KismetMathLibrary.RandomFloatInRange` -2500.0 2500.0))
  (while (and (> (`self.SpawnY`) -500.0) (< (`self.SpawnY`) 500.0))
    (set `self.SpawnY` (`KismetMathLibrary.RandomFloatInRange` -2500.0 2500.0)))
  (`|SpawnActorFromClass` "/Game/Asteroids/UFOSmall_BP.UFOSmall_BP_C" (`KismetMathLibrary.MakeTransform` (`KismetMathLibrary.MakeVector` (`self.SpawnX`) (`self.SpawnY`) 200.0)) "Undefined" "MultiplyWithRoot" null null))

(fn `SpawnUFO`
  (set `self.SpawnX` (`KismetMathLibrary.RandomFloatInRange` -2000.0 2000.0))
  (while (and (> (`self.SpawnX`) -1000.0) (< (`self.SpawnX`) 1000.0))
    (set `self.SpawnX` (`KismetMathLibrary.RandomFloatInRange` -2000.0 2000.0)))
  (set `self.SpawnY` (`KismetMathLibrary.RandomFloatInRange` -2500.0 2500.0))
  (while (and (> (`self.SpawnY`) -500.0) (< (`self.SpawnY`) 500.0))
    (set `self.SpawnY` (`KismetMathLibrary.RandomFloatInRange` -2500.0 2500.0)))
  (`|SpawnActorFromClass` "/Game/Asteroids/UFOParent_BP.UFOParent_BP_C" (`KismetMathLibrary.MakeTransform` (`KismetMathLibrary.MakeVector` (`self.SpawnX`) (`self.SpawnY`) 200.0)) "Undefined" "MultiplyWithRoot" null null))

(fn `UserConstructionScript`)