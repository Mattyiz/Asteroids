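; Enemy bullet for the Asteroids game that aims at the player with slight random inaccuracy.
; On BeginPlay it sets Speed and builds Direction from the unnormalized offset to the second "wrap"-tagged static mesh on the first Player_BP, jittered in X and Y.
; The graph only sets these values, with no movement or hit logic of its own.
; The actor destroys itself after a short delay.
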(event `self.ReceiveBeginPlay`
  (set `self.Speed` 0.01)
  (bind _outactors (`GameplayStatics.GetAllActorsOfClass` "/Game/Asteroids/Player_BP.Player_BP_C"))
  (bind _output_get (set `self.Player` (`|GetArrayItem` _outactors)))
  (bind (_returnvalue_x _returnvalue_y _returnvalue_z) (`KismetMathLibrary.BreakVector` (- (`SceneComponent.K2_GetComponentLocation` (`|GetArrayItem` (`self.GetComponentsByTag` _output_get "/Script/Engine.StaticMeshComponent" "wrap") 1)) (`self.K2_GetActorLocation`))))
  (set `self.Direction` (`KismetMathLibrary.MakeVector` (+ _returnvalue_x (`KismetMathLibrary.RandomFloatInRange` -2.0 2.0)) (+ _returnvalue_y (`KismetMathLibrary.RandomFloatInRange` -2.0 2.0)) _returnvalue_z))
  (`KismetSystemLibrary.Delay` 2.0)
  (`self.K2_DestroyActor`))

(fn `UserConstructionScript`
  (`parent.UserConstructionScript`))