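; TextRenderer_BP is an actor that displays the current score in the Asteroids game through a TextRender component.
; On BeginPlay it finds the first GameManager_BP in the level with GetAllActorsOfClass, caches it and sets the text to its Score.
; Every Tick it polls the manager's Score again and rewrites the text, rather than updating on a change event.
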(event `self.ReceiveBeginPlay`
  (bind _outactors (`GameplayStatics.GetAllActorsOfClass` "/Game/Asteroids/GameManager_BP.GameManager_BP_C"))
  (bind _output_get (set `self.GameManager` (`|GetArrayItem` _outactors)))
  (`TextRenderComponent.K2_SetText` (`self.TextRender`) (`KismetTextLibrary.Conv_IntToText` (`/Game/Asteroids/GameManager_BP.Score` _output_get))))

(event `self.ReceiveTick`
  (params (DeltaSeconds :type "Float (single-precision)"))
  (`TextRenderComponent.K2_SetText` (`self.TextRender`) (`KismetTextLibrary.Conv_IntToText` (`/Game/Asteroids/GameManager_BP.Score` (`self.GameManager`)))))

(fn `UserConstructionScript`)