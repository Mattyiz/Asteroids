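; Small asteroid Blueprint for an Asteroids game, a child class that sets its Speed at BeginPlay before running the parent's logic.
; Its Destroy function finds the GameManager through GetAllActorsOfClass and adds 100 points to both Score and ScoreSinceLife.
; It then destroys the actor without spawning any fragments.
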(event `self.ReceiveBeginPlay`
  (set `self.Speed` 8.0)
  (`parent.ReceiveBeginPlay`))

(fn `Destroy`
  (bind _outactors (`GameplayStatics.GetAllActorsOfClass` "/Game/Asteroids/GameManager.GameManager_C"))
  (bind _output (`|GetArrayItem` _outactors))
  (set `/Game/Asteroids/GameManager.ScoreSinceLife` (+ (`/Game/Asteroids/GameManager.ScoreSinceLife` _output) 100) _output)
  (set `/Game/Asteroids/GameManager.Score` (+ (`/Game/Asteroids/GameManager.Score` _output) 100) _output)
  (`self.K2_DestroyActor`))

(fn `UserConstructionScript`
  (`parent.UserConstructionScript`))