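; Medium asteroid actor that breaks into two small asteroids when destroyed.
; BeginPlay sets its Speed before calling the parent's BeginPlay, and the construction script only calls the parent's.
; Destroy spawns two AsteriodSmall_BP actors at the Sphere component's world transform, adjusting for collisions but always spawning, then destroys the actor itself.
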(event `self.ReceiveBeginPlay`
  (set `self.Speed` 6.0)
  (`parent.ReceiveBeginPlay`))

(fn `Destroy`
  (`|SpawnActorFromClass` "/Game/Asteroids/AsteriodSmall_BP.AsteriodSmall_BP_C" (`SceneComponent.K2_GetComponentToWorld` (`self.Sphere`)) "AdjustIfPossibleButAlwaysSpawn" "MultiplyWithRoot" null null)
  (`|SpawnActorFromClass` "/Game/Asteroids/AsteriodSmall_BP.AsteriodSmall_BP_C" (`SceneComponent.K2_GetComponentToWorld` (`self.Sphere`)) "AdjustIfPossibleButAlwaysSpawn" "MultiplyWithRoot" null null)
  (`self.K2_DestroyActor`))

(fn `UserConstructionScript`
  (`parent.UserConstructionScript`))