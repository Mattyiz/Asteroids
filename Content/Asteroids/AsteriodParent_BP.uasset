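; Base asteroid Blueprint for an Asteroids-style game that drifts across the XY plane and splits when destroyed.
; BeginPlay picks a random, unnormalized XY direction, and Tick offsets the Sphere component by it times Speed each frame, without sweep or delta-time scaling.
; Destroy spawns two AsteriodMid_BP actors at the Sphere's transform, then destroys itself.
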(event `self.ReceiveBeginPlay`
  (set `self.Direction` (`KismetMathLibrary.MakeVector` (`KismetMathLibrary.RandomFloatInRange` -1.0 1.0) (`KismetMathLibrary.RandomFloatInRange` -1.0 1.0))))

(event `self.ReceiveTick`
  (params (DeltaSeconds :type "Float (single-precision)"))
  (`SceneComponent.K2_AddWorldOffset` (`self.Sphere`) (* (`self.Direction`) (`self.Speed`)) false false))

(fn `Destroy`
  (`|SpawnActorFromClass` "/Game/Asteroids/AsteriodMid_BP.AsteriodMid_BP_C" (`SceneComponent.K2_GetComponentToWorld` (`self.Sphere`)) "AdjustIfPossibleButAlwaysSpawn" "MultiplyWithRoot" null null)
  (`|SpawnActorFromClass` "/Game/Asteroids/AsteriodMid_BP.AsteriodMid_BP_C" (`SceneComponent.K2_GetComponentToWorld` (`self.Sphere`)) "AdjustIfPossibleButAlwaysSpawn" "MultiplyWithRoot" null null)
  (`self.K2_DestroyActor`))

(fn `UserConstructionScript`)